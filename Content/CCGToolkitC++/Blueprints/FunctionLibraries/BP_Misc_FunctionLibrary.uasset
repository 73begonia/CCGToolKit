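; Miscellaneous Blueprint function library of shared helpers for the card game toolkit.
; Mouse helpers clamp the cursor within viewport margins, trace under it, or project it to a world distance with a camera-yaw-aligned spawn transform.
; Player helpers resolve self and opponent IDs from human player states or AI pawns, and fetch the local UI manager.
; A widget-transform interpolator eases translation, scale and angle, snapping to the goal and reporting arrival within tolerance.
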(fn BPGetMousePositioninRange
  (params (SizeOffset :type Vector%202D%20Structure) (GlobalEdgeOffset :type Float%20%28single-precision%29) (XEdgeOffset :type Float%20%28single-precision%29) (YEdgeOffset :type Float%20%28single-precision%29))
  (bind (_x _y) (Math|Vector2D|BreakVector2D SizeOffset))
  (bind _returnvalue (Game|GetPlayerController 0))
  (bind _returnvalue_2 (Math|Float|MakeLiteralFloat GlobalEdgeOffset))
  (bind _returnvalue_3 (Viewport|GetViewportSize))
  (bind (_locationx _locationy) (Game|Player|GetMousePosition _returnvalue))
  (bind (_x_2 _y_2) (Math|Vector2D|BreakVector2D _returnvalue_3))
  (return (Math|Vector2D|MakeVector2D (Math|Float|Clamp(Float) _locationx _returnvalue_2 (- (- _x_2 _returnvalue_2) (+ _x XEdgeOffset))) (- (Math|Float|Clamp(Float) _locationy (+ _returnvalue_2 YEdgeOffset) (- (- _y_2 _returnvalue_2) (- _y YEdgeOffset))) YEdgeOffset))))

(fn BPGetPlayerStateReference
  (params (Controller :type Controller%20Object%20Reference))
  (switch int (CallFunction|GetControllerID(ServerOnly) Controller)
    (:1
      (return 1 2))
    (:2
      (return 2 1))))

(fn BPGetControllerID(ServerOnly)
  (params (Controller :type Controller%20Object%20Reference))
  (bind _ascard_game_player_controller_bp (Utilities|Casting|CastToCardGamePlayerController_BP Controller)
    (:then
      (bind _ascard_game_player_state_bp (Utilities|Casting|CastToCardGamePlayerState_BP (Variables|/Script/Engine.Controller|GetPlayerState _ascard_game_player_controller_bp))
        (:then
          (return (Variables|/Script/CCGToolkit.CardGamePlayerState|GetCardGamePlayerId _ascard_game_player_state_bp)))
        (:CastFailed
          _)))
    (:CastFailed
      (bind _ascard_game_aicontroller_bp (Utilities|Casting|CastToCardGameAIController_BP Controller)
        (:then
          (bind _ascard_game_ai_pawn_bp (Utilities|Casting|CastToCardGameAI_Pawn_BP (Pawn|GetControlledPawn _ascard_game_aicontroller_bp)))
          (return (Variables|/Script/CCGToolkit.CardGameAI_Pawn|GetPlayerID _ascard_game_ai_pawn_bp)))
        (:CastFailed
          _))))
  (Development|PrintString 0 "Failed to get Controller")
  (return -1))

(fn BP2DInterptoGoalLocation
  (params (Current%20Transform :type Widget%20Transform%20Structure) (Goal%20Transform :type Widget%20Transform%20Structure) (DeltaTime :type Float%20%28single-precision%29) (InterpSpeed :type Float%20%28single-precision%29))
  (bind (_translation _scale _angle) (Utilities|Struct|BreakWidgetTransform Current%20Transform))
  (bind (_translation_2 _scale_2 _angle_2) (Utilities|Struct|BreakWidgetTransform Goal%20Transform))
  (bind _returnvalue (Class|KismetMathLibrary|Vector2DInterpto _translation _translation_2 DeltaTime InterpSpeed))
  (bind _returnvalue_2 (Math|Vector2D|Vector2DLength _translation_2))
  (bind _returnvalue_3 (Math|Vector2D|Vector2DLength _scale_2))
  (bind _returnvalue_4 (Math|Interpolation|FInterpTo _angle _angle_2 DeltaTime InterpSpeed))
  (bind _returnvalue_5 (Class|KismetMathLibrary|Vector2DInterpto _scale _scale_2 DeltaTime InterpSpeed))
  (bind _returnvalue_6 (Math|Float|Absolute(Float) _angle_2))
  (bind _returnvalue_7 (Math|Vector2D|Vector2DLength _returnvalue))
  (bind _returnvalue_8 (Math|Float|Absolute(Float) _returnvalue_2))
  (bind _returnvalue_9 (Math|Vector2D|Vector2DLength _returnvalue_5))
  (bind _returnvalue_10 (Math|Float|Absolute(Float) _returnvalue_3))
  (bind _returnvalue_11 (Math|Float|Absolute(Float) _returnvalue_4))
  (bind _returnvalue_12 (Math|Float|NearlyEqual(Float) _returnvalue_11 _returnvalue_6 0.001))
  (bind _returnvalue_13 (Math|Float|Absolute(Float) _returnvalue_7))
  (bind _returnvalue_14 (Math|Float|Absolute(Float) _returnvalue_9))
  (bind _returnvalue_15 (Math|Float|NearlyEqual(Float) _returnvalue_13 _returnvalue_8 0.001))
  (bind _returnvalue_16 (Math|Float|NearlyEqual(Float) _returnvalue_14 _returnvalue_10 0.001))
  (bind _returnvalue_17 (Math|Boolean|ANDBoolean _returnvalue_15 _returnvalue_16 _returnvalue_12))
  (bind _returnvalue_18 (not _returnvalue_17))
  (return (Utilities|Struct|MakeWidgetTransform (select _returnvalue_18 _returnvalue _translation_2) (select _returnvalue_18 _returnvalue_5 _scale_2) (select _returnvalue_18 _returnvalue_4 _angle_2)) _returnvalue_17))

(fn BPMouseDistanceinWorldSpace
  (params (Player%20Controller :type Card%20Game%20Player%20Controller%20BP%20Object%20Reference) (Distance :type Float%20%28single-precision%29))
  (bind (_worldlocation _worlddirection) (Game|Player|ConvertMouseLocationToWorldSpace Player%20Controller))
  (bind _returnvalue (* _worlddirection Distance))
  (bind _returnvalue_2 (+ _worldlocation _returnvalue))
  (return _returnvalue_2 (Math|Transform|MakeTransform _returnvalue_2 (.ReturnRotation (Class|MiscFunctionLibrary|GetWorldRotationforPlayer "0, 0, 0")))))

(fn BPMousetoWorldLocation
  (params (Player%20Controller :type Player%20Controller%20Object%20Reference))
  (bind _hitresult (Game|Player|GetHitResultUnderCursorbyChannel Player%20Controller "TraceTypeQuery1" true))
  (return (.hitactor _hitresult) (.location _hitresult)))

(fn BPMouseDistanceinWorldSpace
  (params (Player%20Controller :type Card%20Game%20Player%20Controller%20BP%20Object%20Reference) (Distance :type Float%20%28single-precision%29))
  (bind (_worldlocation _worlddirection) (Game|Player|ConvertMouseLocationToWorldSpace Player%20Controller))
  (bind _returnvalue (* _worlddirection Distance))
  (bind _returnvalue_2 (+ _worldlocation _returnvalue))
  (return _returnvalue_2 (Math|Transform|MakeTransform _returnvalue_2 (.ReturnRotation (CallFunction|GetWorldRotationforPlayer "0, 0, 0")))))

(fn BPGetWorldRotationforPlayer
  (params (OverrideRotationAxis :type Rotator))
  (bind _returnvalue (Game|GetPlayerCameraManager 0))
  (Utilities|IsValid _returnvalue
    (:Is%20Valid
      (return (Math|Rotator|MakeRotator (select (> (.roll OverrideRotationAxis) 0.0) (.pitch OverrideRotationAxis) 0.0) (select (> (.pitch OverrideRotationAxis) 0.0) (.pitch OverrideRotationAxis) 0.0) (select (> (.yaw OverrideRotationAxis) 0.0) (.yaw OverrideRotationAxis) (.yaw (Transformation|GetActorRotation _returnvalue)))) true))
    (:Is%20Not%20Valid
      (return "0, 0, 0" false))))

(fn BPGetPlayerUIManager
  (return (Variables|/Script/CCGToolkit.MyPlayerController|GetUIManager (.AsMy%20Player%20Controller (Utilities|Casting|CastToMyPlayerController (Game|GetPlayerController 0))))))