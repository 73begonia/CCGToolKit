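; Targeting indicator actor for the card game toolkit that draws a drag selection from its own position to a supplied location.
; On BeginPlay it destroys the first instance found if more than one exists.
; SetSelectionProperties shows Target only for valid targets, stretches NarrowCapsule by the distance to Location, and places ToLoacation there.
; Both pieces take their rotation from a look-at toward the mouse's world position, with yaw offset 90 degrees.
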(event EventSetSelectionProperties
  (params (Location :type Vector :default "0, 0, 0") (ValidTarget :type Boolean))
  (bind _returnvalue (Game|GetPlayerController 0))
  (bind _returnvalue_2 (Transformation|GetActorLocation))
  (bind _target (Variables|Default|GetTarget))
  (bind _returnvalue_3 (- Location _returnvalue_2))
  (bind _returnvalue_4 (Class|MiscFunctionLibrary|MousetoWorldLocation _returnvalue))
  (bind _returnvalue_5 (Math|Vector|VectorLength _returnvalue_3))
  (bind _returnvalue_6 (Math|Rotator|FindLookatRotation _returnvalue_2 _returnvalue_4))
  (bind (_roll _pitch _yaw) (Math|Rotator|BreakRotator _returnvalue_6))
  (bind _returnvalue_7 (+ _yaw 9e+01))
  (bind _returnvalue_8 (Math|Rotator|MakeRotator _pitch 0.0 _returnvalue_7))
  (if ValidTarget
    (Rendering|SetVisibility _target true false)
    (else
      (Rendering|SetVisibility _target false false)))
  (Transformation|SetWorldTransform (Variables|Default|GetNarrowCapsule) (Math|Transform|MakeTransform _returnvalue_2 _returnvalue_8 (Math|Vector|MakeVector 1.5 (/ _returnvalue_5 195.0) (/ _returnvalue_5 5e+02))) false false)
  (Transformation|SetWorldTransform (Variables|Default|GetToLoacation) (Math|Transform|MakeTransform Location _returnvalue_8 "2.000000,2.000000,2.000000") false false))

(event EventBeginPlay
  (bind _outactors (Actor|GetAllActorsOfClass "TargetDragSelection_C"))
  (if (> (Utilities|Array|Length _outactors) 1)
    (Actor|DestroyActor (Utilities|Array|Get(acopy) _outactors))))

(fn ConstructionScript)