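; Blueprint for a 3D card actor that moves itself toward a goal transform and offers an enlarged on-screen preview when placed on the board.
; A gated Tick applies interpolated location and rotation, calling ArrivedAtDestinationC when both report done.
; GenerateDescription splits text into fixed-length lines, adding text render components as needed.
; Previews open on delayed hover for desktop and HTML5, or through custom events on iOS and Android.
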(event Custom|Disable%20Mobile%20Card%20Preview
  ;[0.4431 0.9255 1 0.298] iOS / Android - A custom event which can be called to view a larger on-screen (Widget) preview.
  (if (Variables|Default|GetPreviewEnabled)
    (switch Utilities|FlowControl|Switch|SwitchonEPlatform (Variables|Default|GetPlatform)
      (:iOS
        _)
      (:Android
        _))
    (if (Variables|Default|GetbIsPlaced)
      (Utilities|RemoveMouseOverPreview))))

(event Custom|Enable%20Mobile%20Card%20Preview
  (bind _cardpreviewscale (Variables|Default|GetCardPreviewScale))
  ;[0.4431 0.9255 1 0.298] iOS / Android - A custom event which can be called to view a larger on-screen (Widget) preview.
  (if (not (Variables|Default|GetPreviewEnabled))
    (switch Utilities|FlowControl|Switch|SwitchonEPlatform (Variables|Default|GetPlatform)
      (:iOS
        _)
      (:Android
        _))
    (if (Variables|Default|GetbIsPlaced)
      (Variables|Default|SetPreviewEnabled true)
      (Utilities|IsValid (Variables|Default|GetViewCardPreview)
        (:Is%20Valid
          _)
        (:Is%20Not%20Valid
          (bind _returnvalue (UserInterface|CreateWidget "/Game/CCGToolkitC++/Blueprints/Widgets/Gameplay/BP_CardPreviewWidget.BP_CardPreviewWidget_C" (Game|GetPlayerController 0)))
          (bind _output_get (Variables|Default|SetViewCardPreview _returnvalue))))
      (Default|InitiateCardPreview (.AsBP%20Card%20Preview%20Widget (Utilities|Casting|CastToBP_CardPreviewWidget _output_get)) (Variables|Default|GetCardDataTableName) (Variables|Default|GetCardSet) self (select (Variables|Default|GetbIsPlatformMobile) (* _cardpreviewscale 1.5) _cardpreviewscale))
      (UserInterface|Viewport|AddtoViewport (Variables|Default|GetViewCardPreview) 5))))

(event EventBeginPlay)

(event Collision|EventActorBeginOverlap
  (params (OtherActor :type Actor%20Object%20Reference)))

(event EventTick
  (params (DeltaSeconds :type Float%20%28single-precision%29))
  (bind (_returnlocation _returnvalue) (Class|Card3D|InterpSelftoLocation))
  (bind (_returnrotation _returnvalue_2) (Class|Card3D|InterpSelftoRotation))
  ;[0.4431 0.9255 1 0.298] Event Tick
  (Variables|Default|SetCardDeltaTime DeltaSeconds)
  ;[0.4431 0.9255 1 0.298] Gate - InterpTo Location/ Rotation
  (Utilities|FlowControl|Gate true
    (:Exit
      (Transformation|SetActorTransform (Math|Transform|MakeTransform _returnlocation _returnrotation "1,1,1"))
      (if (and _returnvalue _returnvalue_2)
        (Class|Card3D|ArrivedatDestinationC)))))

(event MouseInput|EventActorBeginCursorOver
  (bind _cardpreviewscale (Variables|Default|GetCardPreviewScale))
  ;[0.4431 0.9255 1 0.298] PC / Mac / Linux Events - Allows the user to mouse over a card on the board to view a larger on-screen (Widget) preview.
  (Development|PrintString "Hello")
  (switch Utilities|FlowControl|Switch|SwitchonEPlatform (Variables|Default|GetPlatform)
    (:Windows
      _)
    (:HTML5
      _)
    (:Mac
      _)
    (:Linux
      _))
  (bind _ascard_game_player_controller_bp (Utilities|Casting|CastToCardGamePlayerController_BP (Game|GetPlayerController 0)))
  (if (Utilities|Enum|Equal(Enum) (Variables|/Script/CCGToolkit.CardGamePlayerController|GetPlayerStateEnum _ascard_game_player_controller_bp) "PendingAction") ; Is the player NOT performing any other actions to stop displaying the card preview.
    (if (Variables|Default|GetbIsPlaced) ; Is the card placed on the board?
      (Variables|Default|SetPreviewEnabled true)
      (Utilities|FlowControl|Delay 0.5) ; Short Delay before enabling the preview IF the the card is still moused over. (Stops the preview popping up every card it mouses over)
      (if (and (not (Variables|Default|GetbIsSelected)) (not (Variables|Default|GetbInGraveyard))) ; If the card is selected, do not enable the preview
        (if (Variables|Default|GetPreviewEnabled)
          (Utilities|IsValid (Variables|Default|GetViewCardPreview)
            (:Is%20Valid
              _)
            (:Is%20Not%20Valid
              (bind _returnvalue (UserInterface|CreateWidget "/Game/CCGToolkitC++/Blueprints/Widgets/Gameplay/BP_CardPreviewWidget.BP_CardPreviewWidget_C" (Game|GetPlayerController 0)))
              (bind _output_get (Variables|Default|SetViewCardPreview _returnvalue))))
          (Default|InitiateCardPreview (.AsBP%20Card%20Preview%20Widget (Utilities|Casting|CastToBP_CardPreviewWidget _output_get)) (Variables|Default|GetCardDataTableName) (Variables|Default|GetCardSet) self (select (Variables|Default|GetbIsPlatformMobile) (* _cardpreviewscale 1.5) _cardpreviewscale))
          (UserInterface|Viewport|AddtoViewport (Variables|Default|GetViewCardPreview) 5)
          (else
            (Utilities|RemoveMouseOverPreview)))))))

(event EventGenerateDescription
  (params (DescriptionText :type String))
  (bind _description_text (Variables|Default|GetDescription_Text))
  (Variables|Default|SetCurrentString%20Character 0)
  (for _index (range 0 (/ (Utilities|Array|Length (Utilities|String|GetCharacterArrayfromString DescriptionText)) (Variables|Default|GetMaxDescriptionCharacterLineLength)))
    (if (== _index 0)
      (Rendering|Components|TextRender|SetText _description_text (Utilities|Text|ToText(String) (Utilities|String|GetSubstring DescriptionText (Variables|Default|GetCurrentString%20Character) (Variables|Default|GetMaxDescriptionCharacterLineLength))))
      (Variables|Default|SetCurrentString%20Character (+ (Variables|Default|GetCurrentString%20Character) (Variables|Default|GetMaxDescriptionCharacterLineLength)))
      (else
        (bind _returnvalue (AddComponent|AddTextRenderComponent false (.ReturnValue (|CalculateTextRendererTransform_2 _index DescriptionText))))
        (Rendering|Components|TextRender|SetTextRenderColor _returnvalue (Variables|/Script/Engine.TextRenderComponent|GetTextRenderColor _description_text))
        (Rendering|Components|TextRender|SetWorldSize _returnvalue (Variables|/Script/Engine.TextRenderComponent|GetWorldSize _description_text))
        (Rendering|Components|TextRender|SetText _returnvalue (Utilities|Text|ToText(String) (Utilities|String|GetSubstring (.OutputPin (|CalculateTextRendererTransform_2 _index DescriptionText)) (Variables|Default|GetCurrentString%20Character) (Variables|Default|GetMaxDescriptionCharacterLineLength))))
        (Variables|Default|SetCurrentString%20Character (+ (Variables|Default|GetCurrentString%20Character) (Variables|Default|GetMaxDescriptionCharacterLineLength)))))))

(event MouseInput|EventActorEndCursorOver
  ;[0.4431 0.9255 1 0.298] PC / Mac / Linux Events - Allows the user to mouse over a card on the board to view a larger on-screen (Widget) preview.
  (switch Utilities|FlowControl|Switch|SwitchonEPlatform (Variables|Default|GetPlatform)
    (:Windows
      _)
    (:HTML5
      _)
    (:Mac
      _)
    (:Linux
      _))
  (if (Variables|Default|GetbIsPlaced)
    (Utilities|RemoveMouseOverPreview)))

(event EventOpenGateC
  (bind (_returnlocation _returnvalue) (Class|Card3D|InterpSelftoLocation))
  (bind (_returnrotation _returnvalue_2) (Class|Card3D|InterpSelftoRotation))
  ;[0.4431 0.9255 1 0.298] Events - Open/ Close Gate
  ;[0.4431 0.9255 1 0.298] Gate - InterpTo Location/ Rotation
  (Utilities|FlowControl|Gate true) ; enters at Open
)

(event EventCloseGateC
  (bind (_returnlocation _returnvalue) (Class|Card3D|InterpSelftoLocation))
  (bind (_returnrotation _returnvalue_2) (Class|Card3D|InterpSelftoRotation))
  ;[0.4431 0.9255 1 0.298] Events - Open/ Close Gate
  ;[0.4431 0.9255 1 0.298] Gate - InterpTo Location/ Rotation
  (Utilities|FlowControl|Gate true) ; enters at Close
)

(fn ConstructionScript)

(fn InterpSelftoLocation)

(fn InterpSelftoRotation)