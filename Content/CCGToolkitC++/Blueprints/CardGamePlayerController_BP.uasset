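; Card game player controller that turns touch and mouse input into card interactions and card placement during the player's turn.
; Press, move and release drive a PlayerStateEnum flow: detect and validate locally, then send the interaction or card play through Server functions.
; A held card eases toward the cursor with optional movement-based tilt, refreshed by a Delay loop while placing.
; Off-turn presses spawn a particle, and off-turn movement clears pending states once.
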(event Custom|4.14_OnDragCanceled
  ;[0 0 0] Input Events - Card Placement and Interaction
  (bind _returnvalue (Class|CardGamePlayerController|IsTurnActiveC))
  (if _returnvalue
    (switch Utilities|FlowControl|Switch|SwitchonEPlayerStateEnum (Variables|Default|GetPlayerStateEnum)
      (:CardInteraction
        ;[0 0 0] Check and Run Card Interaction (Step 3)
        (bind _returnvalue_2 (Class|CardGamePlayerController|ValidateInteractionStateC))
        (if _returnvalue_2
          (Class|CardGamePlayerController|ServerRunCardInteractionC (Variables|Default|GetTalkingCard) (Variables|Default|GetRecievingCard) (Variables|Default|GetRecievingPlayer))
          (Class|CardGamePlayerController|CleanCardInteractionStateC :!label _label)
          (Class|CardGamePlayerController|SetInteractionStateC "PendingAction")
          (elif (Variables|Default|GetbIsDragging) ; Is the Player Dragging? If not then this might be a "Click" card selection so do NOT clear the interaction state.
            (goto _label))))
      (:PlacingCard
        ;[0 0 0] Play Card - Drop and Play Card (Step 3)
        (if (Variables|Default|GetbIsValidClientDrop)
          (Class|CardGamePlayerController|ServerPlayCardC (Variables|Default|GetTemp_CreateCardName) (Variables|Default|GetTemp_ChosenCardSet) (Variables|Default|GetTargetCardPlacement) (Variables|Default|GetTempHandIndex) (Transformation|GetActorTransform (Variables|Default|GetPlayCard_Client_Ref)))
          (else
            (Class|CardGamePlayerController|DropCardC false (Variables|Default|GetError_Enum))
            (Actor|DestroyActor (Variables|Default|GetPlayCard_Client_Ref))
            (Variables|Default|SetPlayCard_Client_Ref 0)))
        (Class|CardGamePlayerController|SetInteractionStateC "PendingAction")))))

(event Custom|DestroyClientCard
  ;[0 0 0] Play Card - Drop and Play Card (Step 3)
  (Actor|DestroyActor (Variables|Default|GetPlayCard_Client_Ref))
  (Variables|Default|SetPlayCard_Client_Ref 0)
  (Class|CardGamePlayerController|SetInteractionStateC "PendingAction"))

(event EventBeginPlay
  (Variables|Default|SetbShowMouseCursor true))

(event Input|MouseEvents|LeftMouseButton
  (params (Key :type Key%20Structure :default "None"))
  ;[0 0 0] Input Events - Card Placement and Interaction
  (:Pressed
    (bind _returnvalue (Class|CardGamePlayerController|IsTurnActiveC))
    (if _returnvalue
      ;[0 0 0] Card Interaction - Detect Initial Card Interaction State (Step 1)
      (bind _returnvalue_2 (Class|CardGamePlayerController|CheckPlayerState "Default" "PendingAction" "CardInteraction"))
      (if _returnvalue_2
        (Class|CardGamePlayerController|DetectCardInteractionC))
      (else
        ;[0 0 0] For Fun - Spawn Particle when interacting with the board when not the players turn
        (Effects|SpawnEmitteratLocation 0 (.ReturnValue (Class|MiscFunctionLibrary|MousetoWorldLocation self))))))
  (:Released
    (bind _returnvalue_3 (Class|CardGamePlayerController|IsTurnActiveC))
    (if _returnvalue_3
      (switch Utilities|FlowControl|Switch|SwitchonEPlayerStateEnum (Variables|Default|GetPlayerStateEnum)
        (:CardInteraction
          ;[0 0 0] Check and Run Card Interaction (Step 3)
          (bind _returnvalue_4 (Class|CardGamePlayerController|ValidateInteractionStateC))
          (if _returnvalue_4
            (Class|CardGamePlayerController|ServerRunCardInteractionC (Variables|Default|GetTalkingCard) (Variables|Default|GetRecievingCard) (Variables|Default|GetRecievingPlayer))
            (Class|CardGamePlayerController|CleanCardInteractionStateC :!label _label)
            (Class|CardGamePlayerController|SetInteractionStateC "PendingAction")
            (elif (Variables|Default|GetbIsDragging) ; Is the Player Dragging? If not then this might be a "Click" card selection so do NOT clear the interaction state.
              (goto _label))))
        (:PlacingCard
          ;[0 0 0] Play Card - Drop and Play Card (Step 3)
          (if (Variables|Default|GetbIsValidClientDrop)
            (Class|CardGamePlayerController|ServerPlayCardC (Variables|Default|GetTemp_CreateCardName) (Variables|Default|GetTemp_ChosenCardSet) (Variables|Default|GetTargetCardPlacement) (Variables|Default|GetTempHandIndex) (Transformation|GetActorTransform (Variables|Default|GetPlayCard_Client_Ref)))
            (else
              (Class|CardGamePlayerController|DropCardC false (Variables|Default|GetError_Enum))
              (Actor|DestroyActor (Variables|Default|GetPlayCard_Client_Ref))
              (Variables|Default|SetPlayCard_Client_Ref 0)))
          (Class|CardGamePlayerController|SetInteractionStateC "PendingAction"))))))

(event Input|TouchEvents|InputTouch
  (params (Location :type Vector) (FingerIndex :type ETouchIndex%20Enum))
  ;[0 0 0] Input Events - Card Placement and Interaction
  (:Pressed
    (bind _returnvalue (Class|CardGamePlayerController|IsTurnActiveC))
    (if _returnvalue
      ;[0 0 0] Card Interaction - Detect Initial Card Interaction State (Step 1)
      (bind _returnvalue_2 (Class|CardGamePlayerController|CheckPlayerState "Default" "PendingAction" "CardInteraction"))
      (if _returnvalue_2
        (Class|CardGamePlayerController|DetectCardInteractionC))
      (else
        ;[0 0 0] For Fun - Spawn Particle when interacting with the board when not the players turn
        (Effects|SpawnEmitteratLocation 0 (.ReturnValue (Class|MiscFunctionLibrary|MousetoWorldLocation self))))))
  (:Released
    (bind _returnvalue_3 (Class|CardGamePlayerController|IsTurnActiveC))
    (if _returnvalue_3
      (switch Utilities|FlowControl|Switch|SwitchonEPlayerStateEnum (Variables|Default|GetPlayerStateEnum)
        (:CardInteraction
          ;[0 0 0] Check and Run Card Interaction (Step 3)
          (bind _returnvalue_4 (Class|CardGamePlayerController|ValidateInteractionStateC))
          (if _returnvalue_4
            (Class|CardGamePlayerController|ServerRunCardInteractionC (Variables|Default|GetTalkingCard) (Variables|Default|GetRecievingCard) (Variables|Default|GetRecievingPlayer))
            (Class|CardGamePlayerController|CleanCardInteractionStateC :!label _label)
            (Class|CardGamePlayerController|SetInteractionStateC "PendingAction")
            (elif (Variables|Default|GetbIsDragging) ; Is the Player Dragging? If not then this might be a "Click" card selection so do NOT clear the interaction state.
              (goto _label))))
        (:PlacingCard
          ;[0 0 0] Play Card - Drop and Play Card (Step 3)
          (if (Variables|Default|GetbIsValidClientDrop)
            (Class|CardGamePlayerController|ServerPlayCardC (Variables|Default|GetTemp_CreateCardName) (Variables|Default|GetTemp_ChosenCardSet) (Variables|Default|GetTargetCardPlacement) (Variables|Default|GetTempHandIndex) (Transformation|GetActorTransform (Variables|Default|GetPlayCard_Client_Ref)))
            (else
              (Class|CardGamePlayerController|DropCardC false (Variables|Default|GetError_Enum))
              (Actor|DestroyActor (Variables|Default|GetPlayCard_Client_Ref))
              (Variables|Default|SetPlayCard_Client_Ref 0)))
          (Class|CardGamePlayerController|SetInteractionStateC "PendingAction")))))
  (:Moved
    (bind _returnvalue_5 (Class|CardGamePlayerController|IsTurnActiveC))
    ;[1 1 1] Clear card interaction if it is not/ no longer the players turn
    (if _returnvalue_5
      (Utilities|FlowControl|Sequence
        (:then_0
          (switch Utilities|FlowControl|Switch|SwitchonEPlayerStateEnum (Variables|Default|GetPlayerStateEnum) :!label _label_2
            (:CardInteraction
              ;[0 0 0] Card Interaction - Detect Card Interaction On Move (Step 2)
              (Class|CardGamePlayerController|DetectInteractiononMoveC))
            (:PlacingCard
              ;[0 0 0] Play Card - Select Valid Hold and Drop location - Set the Cards hold location and select a valid placement actor - Step 2
              (CallFunction|SetCardLoacationBP (.Location (CallFunction|MouseDistanceinWorldSpace self (Variables|Default|GetCardHoldDistance))) (.As3DCard (Utilities|Casting|CastTo3DCard (Variables|Default|GetPlayCard_Client_Ref))) (.ReturnRotation (Class|MiscFunctionLibrary|GetWorldRotationforPlayer "0, 0, 0")))
              (Class|CardGamePlayerController|ValidateCardPlacementC (.Hit%20Actor (CallFunction|MousetoWorldLocation self)))
              (Utilities|FlowControl|Delay 0.01)
              (goto _label_2))))
        (:then_1
          (goto _label_3 Reset)))
      (else
        (Utilities|FlowControl|DoOnce false :!label _label_3
          (:Completed
            (Class|CardGamePlayerController|CleanCardInteractionStateC)
            (Class|CardGamePlayerController|CleanCardPlacementState)))))))

(fn ConstructionScript)

(fn Printaa
  (Development|PrintString "aa"))

(fn SetCardLoacationBP
  (params (HoldLocation :type Vector) (Card :type 3D%20Card%20Object%20Reference) (Rotation :type Rotator))
  (bind _returnvalue (Utilities|Time|GetWorldDeltaSeconds))
  (bind _returnvalue_2 (Transformation|GetActorLocation Card))
  ;[0.2113 0.4828 1 0.3] Sets the card "in hand" location and rotation when placing the card on the board.
  (Utilities|IsValid Card
    (:Is%20Valid
      (Transformation|SetActorLocation Card (Math|Interpolation|VInterpTo _returnvalue_2 HoldLocation _returnvalue 1e+01) false false) ; Set the Card in hand's location
      (if (Variables|Default|GetbEnableInHandMovementRotation)
        (Transformation|SetActorRotation Card (Math|Interpolation|RInterpTo (Transformation|GetActorRotation Card) (|GetTargetRotationScaleFactor_2 _returnvalue_2 HoldLocation Rotation) _returnvalue 5.0)) ; Sets rotation of the card based on the movement speed of the mouse.
      ))
    (:Is%20Not%20Valid
      _))
  (return))